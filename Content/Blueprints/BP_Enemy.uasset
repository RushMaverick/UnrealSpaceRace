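; BP_Enemy is an enemy that turns and shoots when it spots the player character.
; Its PawnSensing component filters seen pawns to BP_Char and snaps the actor's rotation to face that pawn.
; After a random delay of up to a second, it spawns a BP_Bullet at its Arrow component's transform.
; BeginPlay only assigns PlayerReference to itself, and the firing logic never uses it.
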(event OnSeePawn(PawnSensing)
  (params (Pawn :type Pawn%20Object%20Reference))
  (Utilities|Casting|CastToBP_Char Pawn)
  (Transformation|SetActorRotation (Math|Rotator|FindLookatRotation (Transformation|GetActorLocation) (Transformation|GetActorLocation Pawn)))
  (Utilities|FlowControl|Delay (Math|Random|RandomFloat))
  (Game|SpawnActorfromClass "/Game/Blueprints/BP_Bullet.BP_Bullet_C" (Transformation|GetWorldTransform (Variables|Default|GetArrow)) "Undefined" "MultiplyWithRoot" 0 0))

(event EventBeginPlay
  (Variables|Default|SetPlayerReference (Variables|Default|GetPlayerReference)))

(event Collision|EventActorBeginOverlap
  (params (OtherActor :type Actor%20Object%20Reference)))

(fn ConstructionScript)